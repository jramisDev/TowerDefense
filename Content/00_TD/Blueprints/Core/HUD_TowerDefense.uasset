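; Tower defense HUD that shows and hides the radial building selection menu and forwards directional input to it.
; ToggleBuildingMenu lazily creates and reuses WBP_RadialSelector, adds it to the player screen, and pairs it with the IMC_BuildingSelection Enhanced Input mapping context.
; It tracks a single active widget, which receives direction messages from SendDirectionToUI and is cleared only if it matches the widget being closed.
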(event `SendDirectionToUI`
  (params (Direction :type "/Game/00_TD/Blueprints/Enums/E_Directions Enum" :default "NewEnumerator0"))
  (bind _activewidget (`self.ActiveWidget`)
    (:`then`
      (message `/Game/00_TD/Blueprints/Interfaces/BPI_WidgetAction.SendDirection` _activewidget Direction))
    (:`else`)))

(fn `SetActiveWidget`
  (params (ActiveWidget :type "UserWidget Object Reference"))
  (set `self.ActiveWidget` ActiveWidget))

(fn `ToggleBuildingMenu`
  (params (OnOff :type Boolean))
  (bind _wbp_radial_selector (`self.WBP Radial Selector`))
  (if OnOff
    (`self.WBP Radial Selector`
      (:`then`
        _)
      (:`else`
        (bind _returnvalue (`|CreateWidget` "/Game/00_TD/UI/WBP_RadialSelector.WBP_RadialSelector_C"))
        (set `self.WBP Radial Selector` _returnvalue)))
    (`UserWidget.AddToPlayerScreen` _wbp_radial_selector 0)
    (`self.SetActiveWidget` _wbp_radial_selector)
    (`EnhancedInputSubsystemInterface.AddMappingContext` (pcsubsystem `EnhancedInputLocalPlayerSubsystem` (`self.GetOwningPlayerController`)) "/Game/00_TD/Inputs/IMC_BuildingSelection.IMC_BuildingSelection" 0 (struct))
    (else
      (bind _wbp_radial_selector_2 (`self.WBP Radial Selector`)
        (:`then`
          (`Widget.RemoveFromParent` _wbp_radial_selector_2)
          (`self.UnSetActiveWidget` _wbp_radial_selector_2))
        (:`else`
          _))
      (`EnhancedInputSubsystemInterface.RemoveMappingContext` (pcsubsystem `EnhancedInputLocalPlayerSubsystem` (`self.GetOwningPlayerController`)) "/Game/00_TD/Inputs/IMC_BuildingSelection.IMC_BuildingSelection" (struct)))))

(fn `UnSetActiveWidget`
  (params (OldActiveWidget :type "UserWidget Object Reference"))
  (bind _activewidget (`self.ActiveWidget`)
    (:`then`
      (if (== _activewidget OldActiveWidget)
        (set `self.ActiveWidget` null)))
    (:`else`)))

(fn `UserConstructionScript`)