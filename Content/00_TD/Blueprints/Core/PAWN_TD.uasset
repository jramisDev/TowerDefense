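; PAWN_TD is a player pawn that moves on the horizontal plane and projects a widget cursor onto the surface the camera faces.
; IA_Movement feeds its 2D input straight into FloatingPawnMovement as a world-space vector, then line traces along the camera's forward on Visibility.
; On a hit, WidgetCursor sits slightly off the surface and faces along its normal, with a debug arrow drawn.
; The cursor updates only when movement input fires.
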(event `EnhancedInput|/Game/00_TD/Inputs/IA_Movement`
  (params (ActionValue :type "Vector2D Structure") (ElapsedSeconds :type "Float (double-precision)") (TriggeredSeconds :type "Float (double-precision)") (InputAction :type "InputAction Object Reference" :default "/Game/00_TD/Inputs/IA_Movement.IA_Movement"))
  (bind _camera (`self.Camera`))
  (bind _returnvalue (`SceneComponent.K2_GetComponentLocation` _camera))
  (:`Triggered`
    (`PawnMovementComponent.AddInputVector` (`self.FloatingPawnMovement`) (`KismetMathLibrary.Conv_Vector2DToVector` ActionValue) false)
    (bind (_outhit _returnvalue_2) (`KismetSystemLibrary.LineTraceSingle` _returnvalue (+ _returnvalue (* (`SceneComponent.GetForwardVector` _camera) 200000.0)) "TraceTypeQuery1"))
    (if _returnvalue_2
      (bind (_bblockinghit _binitialoverlap _time _distance _location _impactpoint _normal) (`GameplayStatics.BreakHitResult` _outhit))
      (bind _returnvalue_3 (+ _location (* _normal 10.0)))
      (`SceneComponent.K2_SetWorldLocation` (`self.WidgetCursor`) _returnvalue_3 false false)
      (`KismetSystemLibrary.DrawDebugArrow` _location _returnvalue_3 3.0 (struct :`R` 1.0 :`A` 1.0) 1.0 3.0)
      (`SceneComponent.K2_SetWorldRotation` (`self.WidgetCursor`) (`KismetMathLibrary.FindLookAtRotation` _location _returnvalue_3) false false))))

(fn `UserConstructionScript`)