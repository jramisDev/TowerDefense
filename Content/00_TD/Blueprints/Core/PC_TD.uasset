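; Player controller for the tower defense game that handles tower placement through Enhanced Input.
; Opening the build menu line-traces via the cached TD pawn and spawns a preview tower at the hit, currently hardcoded to the fire tower.
; Confirm spawns the real tower class at the preview's child actor transform and removes the preview, with no validity check on placement.
; Cancel simply destroys the preview.
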(event `self.ReceiveBeginPlay`
  (`EnhancedInputSubsystemInterface.AddMappingContext` (subsystem `EnhancedInputLocalPlayerSubsystem`) "/Game/00_TD/Inputs/IMC_Game.IMC_Game" 0 (struct))
  (`WidgetBlueprintLibrary.SetFocusToGameViewport`))

(event `EnhancedInput|/Game/00_TD/Inputs/IA_OpenBuildMenu`
  (params (ActionValue :type Boolean) (ElapsedSeconds :type "Float (double-precision)") (TriggeredSeconds :type "Float (double-precision)") (InputAction :type "InputAction Object Reference" :default "/Game/00_TD/Inputs/IA_OpenBuildMenu.IA_OpenBuildMenu"))
  (:`Completed`
    (bind (_outhit _returnvalue) (`/Game/00_TD/Blueprints/Core/PAWN_TD.MakeLineTrace` (`self.GetPawnRef`) "TraceTypeQuery3"))
    (if _returnvalue
      (bind _returnvalue_2 (`|SpawnActorFromClass` "/Game/00_TD/Blueprints/Towers/BP_PreviewTower.BP_PreviewTower_C" (`KismetMathLibrary.MakeTransform` (`.Location` (`GameplayStatics.BreakHitResult` _outhit))) "Undefined" "MultiplyWithRoot" self "/Game/00_TD/Blueprints/Towers/BP_FireTower.BP_FireTower_C" null))
      (set `self.Preview Tower` _returnvalue_2))))

(event `EnhancedInput|/Game/00_TD/Inputs/IA_Confirm`
  (params (ActionValue :type Boolean) (ElapsedSeconds :type "Float (double-precision)") (TriggeredSeconds :type "Float (double-precision)") (InputAction :type "InputAction Object Reference" :default "/Game/00_TD/Inputs/IA_Confirm.IA_Confirm"))
  (:`Started`
    (bind _preview_tower (`self.Preview Tower`)
      (:`then`
        (if true
          (`|SpawnActorFromClass` (`/Game/00_TD/Blueprints/Towers/BP_PreviewTower.ClassToSpawn` _preview_tower) (`SceneComponent.K2_GetComponentToWorld` (`/Game/00_TD/Blueprints/Towers/BP_PreviewTower.ChildActor` _preview_tower)) "Undefined" "MultiplyWithRoot" null false null)
          (`self.K2_DestroyActor` (`self.Preview Tower`))
          (set `self.Preview Tower` null)))
      (:`else`))))

(event `EnhancedInput|/Game/00_TD/Inputs/IA_Cancel`
  (params (ActionValue :type Boolean) (ElapsedSeconds :type "Float (double-precision)") (TriggeredSeconds :type "Float (double-precision)") (InputAction :type "InputAction Object Reference" :default "/Game/00_TD/Inputs/IA_Cancel.IA_Cancel"))
  (:`Completed`
    (bind _preview_tower (`self.Preview Tower`)
      (:`then`
        (`self.K2_DestroyActor` _preview_tower)
        (set `self.Preview Tower` null))
      (:`else`))))

(fn `GetPawnRef`
  (returns (`As PAWN TD` :type "/Game/00_TD/Blueprints/Core/PAWN_TD Object Reference"))
  (`self.As PAWN TD`
    (:`then`
      _)
    (:`else`
      (bind _aspawn_td (cast `/Game/00_TD/Blueprints/Core/PAWN_TD` (`self.K2_GetPawn`)))
      (set `self.As PAWN TD` _aspawn_td)))
  (return (`self.As PAWN TD`)))

(fn `UserConstructionScript`)