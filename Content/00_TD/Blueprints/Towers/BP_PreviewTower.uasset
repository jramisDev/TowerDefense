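; Placement preview for a tower in a tower defense game, showing the class to spawn as a child actor.
; Each tick it uses the owning PC_TD's pawn line trace to set ValidTerrain and, on a hit, moves to that point with zero rotation.
; It then box traces at the child's bounds origin, ignoring the child, to set NotOcupped, with debug drawing left on.
; GetPCRef lazily caches the owner cast.
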(event `self.ReceiveBeginPlay`
  (`ChildActorComponent.SetChildActorClass` (`self.ChildActor`) (`self.ClassToSpawn`)))

(event `self.ReceiveTick`
  (params (DeltaSeconds :type "Float (single-precision)"))
  (bind _childactor (`ChildActorComponent.ChildActor` (`self.ChildActor`)))
  (bind _origin (`self.GetActorBounds` _childactor true false))
  (bind (_outhit _returnvalue) (`/Game/00_TD/Blueprints/Core/PAWN_TD.MakeLineTrace` (`/Game/00_TD/Blueprints/Core/PC_TD.GetPawnRef` (`self.GetPCRef`)) "TraceTypeQuery3"))
  (set `self.ValidTerrain` _returnvalue)
  (if _returnvalue
    (`self.K2_SetActorLocationAndRotation` (`.Location` (`GameplayStatics.BreakHitResult` _outhit)) (struct))
    (bind (_outhit_2 _returnvalue_2) (`KismetSystemLibrary.BoxTraceSingle` _origin _origin (50.0 50.0 50.0) (struct) "TraceTypeQuery4" false (`|MakeArray` _childactor) "ForDuration"))
    (set `self.NotOcupped` (not _returnvalue_2))))

(fn `GetPCRef`
  (returns (`As PC TD` :type "/Game/00_TD/Blueprints/Core/PC_TD Object Reference"))
  (`self.As PC TD`
    (:`then`
      _)
    (:`else`
      (bind _aspc_td (cast `/Game/00_TD/Blueprints/Core/PC_TD` (`self.GetOwner`)))
      (set `self.As PC TD` _aspc_td)))
  (return (`self.As PC TD`)))

(fn `UserConstructionScript`)