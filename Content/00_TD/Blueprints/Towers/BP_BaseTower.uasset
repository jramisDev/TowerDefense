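; Base tower for a tower defense game that automatically fires at enemies inside its detection area.
; Overlap events and an initial scan maintain a target list, and new entries trigger Attack.
; Attack glides a spawned projectile to the first target, then destroys it and applies damage, while a cooldown timer re-triggers firing.
; Preview towers ignore detection collision, and the construction script disables collision responses on visual mesh children.
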(event `self.ReceiveBeginPlay`
  (if (`self.Preview`)
    (`PrimitiveComponent.SetCollisionResponseToAllChannels` (`self.EnemyDetection`) "ECR_Ignore")
    (else
      (`self.RefreshDetectionArea`))))

(event `self.EnemyDetection.OnComponentBeginOverlap`
  (params (OverlappedComponent :type "PrimitiveComponent Object Reference") (OtherActor :type "Actor Object Reference") (OtherComp :type "PrimitiveComponent Object Reference") (OtherBodyIndex :type Integer) (bFromSweep :type Boolean) (SweepResult :type "HitResult Structure (by ref)"))
  (bind _asbp_enemy_base (cast `/Game/00_TD/Blueprints/Enemies/BP_EnemyBase` OtherActor))
  (`self.AddEnemySpotted` _asbp_enemy_base))

(event `self.EnemyDetection.OnComponentEndOverlap`
  (params (OverlappedComponent :type "PrimitiveComponent Object Reference") (OtherActor :type "Actor Object Reference") (OtherComp :type "PrimitiveComponent Object Reference") (OtherBodyIndex :type Integer))
  (bind _asbp_enemy_base (cast `/Game/00_TD/Blueprints/Enemies/BP_EnemyBase` OtherActor))
  (`self.TargetLost` _asbp_enemy_base))

(event `Attack`
  (bind _output (`|GetArrayItem` (`self.Targets`)))
  (if (and (`KismetArrayLibrary.Array_IsNotEmpty` (`self.Targets`)) (`self.ReadyToFire`))
    (bind _returnvalue (`|SpawnActorFromClass` "/Game/00_TD/Blueprints/Towers/Attacks/BP_ProjectileBase.BP_ProjectileBase_C" (`KismetMathLibrary.MakeTransform` (`self.K2_GetActorLocation`)) "Undefined" "MultiplyWithRoot" null null))
    (`|ExecutionSequence`
      (:`then_0`
        (`KismetSystemLibrary.MoveComponentTo` (`Actor.RootComponent` _returnvalue) (`self.K2_GetActorLocation` _output) (struct) false false 0.1)
        (`self.K2_DestroyActor` _returnvalue)
        (`GameplayStatics.ApplyDamage` _output 1.0))
      (:`then_1`
        (`KismetSystemLibrary.K2_SetTimerDelegate` (delegate `SetReadyToFire`) 1.0)
        (set `self.ReadyToFire` false)))
    (else
      (`KismetSystemLibrary.K2_ClearAndInvalidateTimerHandle` (`self.AttackingTimer`)))))

(event `SetReadyToFire`
  (set `self.ReadyToFire` true)
  (`self.Attack`))

(fn `AddEnemySpotted`
  (params (Enemy :type "/Game/00_TD/Blueprints/Enemies/BP_EnemyBase Object Reference (by ref)"))
  (`KismetArrayLibrary.Array_AddUnique` (`self.Targets`) Enemy)
  (`self.Attack`))

(fn `RefreshDetectionArea`
  (locals (EnemysBase :type "Array of Actor Object Reference"))
  (`KismetArrayLibrary.Array_Clear` (`self.Targets`))
  (bind _output_get (set `local.EnemysBase` (`PrimitiveComponent.GetOverlappingActors` (`self.EnemyDetection`) "/Game/00_TD/Blueprints/Enemies/BP_EnemyBase.BP_EnemyBase_C")))
  (for _array_element _output_get
    (bind _asbp_enemy_base (cast `/Game/00_TD/Blueprints/Enemies/BP_EnemyBase` _array_element))
    (`self.AddEnemySpotted` _asbp_enemy_base)))

(fn `TargetLost`
  (params (Enemy :type "/Game/00_TD/Blueprints/Enemies/BP_EnemyBase Object Reference (by ref)"))
  (`KismetArrayLibrary.Array_RemoveItem` (`self.Targets`) Enemy))

(fn `UserConstructionScript`
  (locals (Childrens :type "Array of SceneComponent Object Reference"))
  (bind _output_get (set `local.Childrens` (`SceneComponent.GetChildrenComponents` (`self.VisualMesh`) false)))
  (for _array_element _output_get
    (bind _asprimitive_component (cast `PrimitiveComponent` _array_element))
    (`PrimitiveComponent.SetCollisionResponseToAllChannels` _asprimitive_component "ECR_Ignore")))